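; BP_MainTerrain3 is a terrain actor that configures parameters for map generation covering size, city plan, water, rivers and roads.
; On BeginPlay it clears Is2d, builds DebugParams with only wall drawing enabled among the road, wall and main flags, and sets MapParams as initialized.
; PrintDebug then prints the map settings on screen for inspection.
; No generation logic appears in this graph, and the construction script is empty.
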(event EventBeginPlay
  (Variables|Default|Setis_2d false)
  (Variables|Default|SetDebugParams (Utilities|Struct|MakeDebugParams false true false))
  (Variables|Default|SetMapParams (Utilities|Struct|MakeMapParams 8e+01 1.5e+02 45.0 1e+01 7e+01 95.0 2e+01 6.0 3.0 "radial_circle" "process_houses" "river" 4e+03 4e+03 42.0 1e+02 8e+01 true))
  (CallFunction|PrintDebug))

(event Collision|EventActorBeginOverlap
  (params (OtherActor :type Actor%20Object%20Reference)))

(event EventTick
  (params (DeltaSeconds :type Float%20%28single-precision%29)))

(fn ConstructionScript)

(fn PrintDebug
  (bind _mapparams (Variables|Default|GetMapParams))
  (bind (_av_river_length _max_river_length _min_new_road_length _min_road_length _av_road_length _max_road_length _river_road_distance _main_road_width _road_width _city_plan _draw_stage _water_type _x_size _y_size _road_left_chance _road_forward_chance _road_right_chance) (Utilities|Struct|BreakMapParams _mapparams))
  (Development|PrintString (Utilities|String|Append "X Size: " (Utilities|String|ToString(Float) _x_size)) true true "(R=0.000000,G=0.660000,B=1.000000,A=1.000000)" 5e+01)
  (Development|PrintString (Utilities|String|Append "Y Size: " (Utilities|String|ToString(Float) _y_size)) true true "(R=0.000000,G=0.660000,B=1.000000,A=1.000000)" 5e+01)
  (Development|PrintString (Utilities|String|Append "City plan:" (Utilities|String|EnumtoString _city_plan)) true true "(R=0.000000,G=0.660000,B=1.000000,A=1.000000)" 5e+01)
  (Development|PrintString (Utilities|String|Append "water type: " (Utilities|String|EnumtoString _water_type)) true true "(R=0.000000,G=0.660000,B=1.000000,A=1.000000)" 5e+01)
  (Development|PrintString (Utilities|String|Append "Av River Length" (Utilities|String|ToString(Float) _av_river_length)) true true "(R=0.000000,G=0.660000,B=1.000000,A=1.000000)" 5e+01)
  (Development|PrintString (Utilities|String|Append "Max river length" (Utilities|String|ToString(Float) _max_river_length)) true true "(R=0.000000,G=0.660000,B=1.000000,A=1.000000)" 5e+01)
  (Development|PrintString (Utilities|String|Append "min new road length: " (Utilities|String|ToString(Float) _min_new_road_length)) true true "(R=0.000000,G=0.660000,B=1.000000,A=1.000000)" 5e+01)
  (Development|PrintString (Utilities|String|Append "min road length: " (Utilities|String|ToString(Float) _min_road_length)) true true "(R=0.000000,G=0.660000,B=1.000000,A=1.000000)" 5e+01)
  (Development|PrintString (Utilities|String|Append "av road length: " (Utilities|String|ToString(Float) _av_road_length)) true true "(R=0.000000,G=0.660000,B=1.000000,A=1.000000)" 5e+01)
  (Development|PrintString (Utilities|String|Append "Max road length: " (Utilities|String|ToString(Float) _max_road_length)) true true "(R=0.000000,G=0.660000,B=1.000000,A=1.000000)" 5e+01)
  (Development|PrintString (Utilities|String|Append "River road distance: " (Utilities|String|ToString(Float) _river_road_distance)) true true "(R=0.000000,G=0.660000,B=1.000000,A=1.000000)" 5e+01)
  (Development|PrintString (Utilities|String|Append "Road left chance: " (Utilities|String|ToString(Float) _road_left_chance)) true true "(R=0.000000,G=0.660000,B=1.000000,A=1.000000)" 5e+01)
  (Development|PrintString (Utilities|String|Append "road forward chance: " (Utilities|String|ToString(Float) _road_forward_chance)) true true "(R=0.000000,G=0.660000,B=1.000000,A=1.000000)" 5e+01)
  (Development|PrintString (Utilities|String|Append "road right chance: " (Utilities|String|ToString(Float) _road_right_chance)) true true "(R=0.000000,G=0.660000,B=1.000000,A=1.000000)" 5e+01))