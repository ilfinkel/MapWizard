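; BP_MainTerrain is a terrain actor that sets up city map and debug parameters when play begins.
; BeginPlay casts the Game Instance to BP_Map_Parameters, prints its map X size and feeds it into MapParams alongside hardcoded layout and road settings.
; It also sets debug draw flags and enables Is2d.
; No generation logic is in this graph; leftover debug prints are unconnected and the construction script is empty.
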(event EventBeginPlay
  (bind _asbp_map_parameters (Utilities|Casting|CastToBP_Map_Parameters (Game|GetGameInstance)))
  (Development|PrintString (Utilities|String|ToString(Float) (Variables|/Game/BP_Map_Parameters.BP_Map_Parameters_C|GetSize_map_X _asbp_map_parameters)))
  (Variables|Default|SetMapParams (Utilities|Struct|MakeMapParams 8e+01 1.5e+02 45.0 1e+01 7e+01 95.0 2e+01 "radial_circle" "process_houses" "river" (Variables|/Game/BP_Map_Parameters.BP_Map_Parameters_C|GetSize_map_X _asbp_map_parameters) 1e+03 75.0 1e+02 4e+01))
  (Variables|Default|SetDebugParams (Utilities|Struct|MakeDebugParams true false true))
  (Variables|Default|Setis_2d true))

(event Collision|EventActorBeginOverlap
  (params (OtherActor :type Actor%20Object%20Reference)))

(event EventTick
  (params (DeltaSeconds :type Float%20%28single-precision%29)))

(fn ConstructionScript)