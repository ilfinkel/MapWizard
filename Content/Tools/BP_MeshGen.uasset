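; BP_MeshGen is a Geometry Script generator actor that builds a displaced mesh from a source static mesh.
; On rebuild, it copies the source into the dynamic mesh and applies PN tessellation driven by Smoothness.
; With a valid displacement texture, it displaces by Height, smooths iteratively, recomputes normals, then plane-cuts at CutLocation with the cut side flipped.
; Without that texture, the chain stops after tessellation.
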(event EventBeginPlay)

(event Collision|EventActorBeginOverlap
  (params (OtherActor :type Actor%20Object%20Reference)))

(event EventTick
  (params (DeltaSeconds :type Float%20%28single-precision%29)))

(event Events|EventOnRebuildGeneratedMesh
  (params (TargetMesh :type Dynamic%20Mesh%20Object%20Reference))
  (bind _sourcemesh (Variables|Default|GetSourceMesh)
    (:then
      (bind _returnvalue (Class|GeometryScriptLibraryStaticMeshFunctions|CopyMeshfromStaticMeshV2 :FromStaticMeshAsset _sourcemesh :ToDynamicMesh TargetMesh :Debug 0)
        (:Success
          (bind _returnvalue_2 (Class|GeometryScriptLibraryMeshSubdivideFunctions|ApplyPNTessellation :TargetMesh _returnvalue :TessellationLevel (Variables|Default|GetSmoothness) :Debug 0))
          (bind _displacemap (Variables|Default|GetDisplaceMap)
            (:then
              (bind _returnvalue_3 (Class|GeometryScriptLibraryMeshDeformFunctions|ApplyDisplacefromTextureMap :TargetMesh _returnvalue_2 :Texture _displacemap :Options (Utilities|Struct|MakeGeometryScriptDisplaceFromTextureOptions (Variables|Default|GetHeight) "(X=1.000000,Y=1.000000)" "(X=0.000000,Y=0.000000)" 0.5 0 "FullMeshSelection") :Debug 0))
              (bind _returnvalue_4 (Class|GeometryScriptLibraryMeshDeformFunctions|ApplyIterativeSmoothingtoMesh :TargetMesh _returnvalue_3 :Debug 0))
              (bind _returnvalue_5 (GeometryScript|Normals|RecomputeNormals :TargetMesh _returnvalue_4 :Debug 0))
              (Class|GeometryScriptLibraryMeshBooleanFunctions|ApplyMeshPlaneCut _returnvalue_5 (Math|Transform|MakeTransform (Variables|Default|GetCut%20Location) "0, 0, 0" "1.000000,1.000000,1.000000") (Utilities|Struct|MakeGeometryScriptMeshPlaneCutOptions true -1 true true 1.0) 0))
            (:else)))))
    (:else)))

(fn ConstructionScript)